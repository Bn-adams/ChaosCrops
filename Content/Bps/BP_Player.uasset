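; Player pawn for a timed 2D farming game that moves, waters and harvests crops, creates the HUD and opens the end screen when time runs out.
; Watering swaps overlapped waterable beets and potatoes for grown versions spawned at the player's position, and hoeing harvests those into a crop count.
; The capped watering can refills near a well.
; An animation enum, set by keys and delayed action events, selects the Paper2D flipbook every Tick.
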(event `NoMoretime`
  (if (not (> (`self.GameTimer`) 0))
    (`self.GameEnd`)))

(event `self.ReceiveBeginPlay`
  (set `self.WaterAmount` 5)
  (bind _returnvalue (`|CreateWidget` "/Game/interface/Player_HUD.Player_HUD_C"))
  (`UserWidget.AddToViewport` _returnvalue 0)
  (`KismetSystemLibrary.K2_SetTimerDelegate` (delegate `EverySecond`) 1.0 true))

(event `EverySecond`
  (set `self.GameTimer` (- (`self.GameTimer`) 1)))

(event `self.ReceiveTick`
  (params (DeltaSeconds :type "Float (single-precision)"))
  (`self.AniHandler`)
  (`self.NoMoretime`))

(event `InputAxis|MoveRight`
  (params (AxisValue :type "Float (single-precision)"))
  ;[1 1 1] Movement
  (`self.AddMovementInput` (1.0 0.0 0.0) AxisValue))

(event `InputAction|Hoeing`
  (params (Key :type "Key Structure"))
  (:`Pressed`
    (`self.Hoeing Animation`)
    (bind _returnvalue (`GameplayStatics.GetActorOfClass` "BP_Player_C"))
    (`|ExecutionSequence`
      (:`then_0`
        (for _array_element (`self.GetOverlappingActors` _returnvalue "/Game/Bps/BP_Beet2.BP_Beet2_C")
          (`self.K2_DestroyActor` _array_element)
          (set `self.CropAmount` (+ (`self.CropAmount`) 1) :!label _label)
          (if (> (`self.CropAmount`) (`self.CropGoal`))
            _)))
      (:`then_1`
        (for _array_element_2 (`self.GetOverlappingActors` _returnvalue "/Game/Bps/BP_Potato2.BP_Potato2_C")
          (`self.K2_DestroyActor` _array_element_2)
          (goto _label))))))

(event `InputAction|Watering`
  (params (Key :type "Key Structure"))
  ;[1 1 1] Watering
  (:`Pressed`
    (if (> (`self.WaterAmount`) 0)
      (`self.Watering animation`)
      (set `self.WaterAmount` (- (`self.WaterAmount`) 1))
      (`self.Water Beet`)
      (`self.Water Potato`)
      (else
        (`KismetSystemLibrary.PrintString` "Go to the well for more water ")))))

(event `InputAxis|MoveUp`
  (params (AxisValue :type "Float (single-precision)"))
  ;[1 1 1] Movement
  (`self.AddMovementInput` (0.0 -1.0 0.0) AxisValue))

(event `Water Beet`
  ;[1 1 1] Watering
  (bind _returnvalue (`GameplayStatics.GetActorOfClass` "BP_Player_C"))
  (for _array_element (`self.GetOverlappingActors` _returnvalue "/Game/Bps/BP_Beet1.BP_Beet1_C")
    (bind _asbp_beet_1 (cast `/Game/Bps/BP_Beet1` _array_element))
    (if (`/Game/Bps/BP_Beet1.is Waterable` _asbp_beet_1)
      (`self.K2_DestroyActor` _array_element)
      (`|SpawnActorFromClass` "/Game/Bps/BP_Beet2.BP_Beet2_C" (`KismetMathLibrary.Conv_VectorToTransform` (`self.K2_GetActorLocation` _returnvalue)) "Undefined" "OverrideRootScale" null null))))

(event `AniHandler`
  ;[1 1 1] Set enumarator flipbooks
  (switch `/Game/Assets/FlipBooks/AnimationHandler` (`self.AniState`)
    (:`NewEnumerator0`
      (`PaperFlipbookComponent.SetFlipbook` (`self.PaperFlipbook`) "/Game/Assets/FlipBooks/FMan_Idle.FMan_Idle"))
    (:`NewEnumerator5`
      (`PaperFlipbookComponent.SetFlipbook` (`self.PaperFlipbook`) "/Game/Assets/FlipBooks/Farm_man_Idle_Left1.Farm_man_Idle_Left1"))
    (:`NewEnumerator1`
      (`PaperFlipbookComponent.SetFlipbook` (`self.PaperFlipbook`) "/Game/Assets/FlipBooks/FMan_Run.FMan_Run"))
    (:`NewEnumerator4`
      (`PaperFlipbookComponent.SetFlipbook` (`self.PaperFlipbook`) "/Game/Assets/FlipBooks/Farm_man_Run_Left1.Farm_man_Run_Left1"))
    (:`NewEnumerator2`
      (`PaperFlipbookComponent.SetFlipbook` (`self.PaperFlipbook`) "/Game/Assets/FlipBooks/Farm_man_Watering1.Farm_man_Watering1"))
    (:`NewEnumerator3`
      (`PaperFlipbookComponent.SetFlipbook` (`self.PaperFlipbook`) "/Game/Assets/FlipBooks/Farm_man_Hoe1.Farm_man_Hoe1"))
    (:`NewEnumerator6`
      (`PaperFlipbookComponent.SetFlipbook` (`self.PaperFlipbook`) "/Game/Assets/FlipBooks/Farm_man_Watering_Left1.Farm_man_Watering_Left1"))
    (:`NewEnumerator7`
      (`PaperFlipbookComponent.SetFlipbook` (`self.PaperFlipbook`) "/Game/Assets/FlipBooks/Farm_man_Hoe_LEft1.Farm_man_Hoe_LEft1"))))

(event `Water Potato`
  ;[1 1 1] Watering
  (bind _returnvalue (`GameplayStatics.GetActorOfClass` "BP_Player_C"))
  (for _array_element (`self.GetOverlappingActors` _returnvalue "/Game/Bps/BP_Potato1.BP_Potato1_C")
    (bind _asbp_potato_1 (cast `/Game/Bps/BP_Potato1` _array_element))
    (if (`/Game/Bps/BP_Potato1.is Waterable` _asbp_potato_1)
      (`self.K2_DestroyActor` _array_element)
      (`|SpawnActorFromClass` "/Game/Bps/BP_Potato2.BP_Potato2_C" (`KismetMathLibrary.Conv_VectorToTransform` (`self.K2_GetActorLocation` _returnvalue)) "Undefined" "OverrideRootScale" null null))))

(event `WaterCheck`
  ;[1 1 1] WaterCheck
  (if (> (`self.WaterAmount`) 10)
    (set `self.WaterAmount` (- (`self.WaterAmount`) 1))
    (`KismetSystemLibrary.PrintString` "Too Much Water")))

(event `InputAction|FillingWater`
  (params (Key :type "Key Structure"))
  ;[1 1 1] Fill Watering can
  (:`Pressed`
    (if (`self.PlayerNearWell`)
      (set `self.WaterAmount` (+ (`self.WaterAmount`) 1))
      (`self.WaterCheck`)
      (else
        (`KismetSystemLibrary.PrintString` "You Need to be Near a Water well")))))

(event `Key|D`
  (params (Key :type "Key Structure"))
  ;[1 1 1] Animations
  (:`Pressed`
    (set `self.AniState` "NewEnumerator1")
    (set `self.IsRunningLeft` false)
    (set `self.IsRunningRight` true))
  (:`Released`
    (set `self.AniState` "NewEnumerator0")))

(event `Watering animation`
  ;[1 1 1] Animations
  ;;[1 1 1] Watering can
  (`|ExecutionSequence`
    (:`then_0`
      (if (`self.IsRunningLeft`)
        (set `self.AniState` "NewEnumerator6")
        (`KismetSystemLibrary.Delay` 0.5)
        (set `self.AniState` "NewEnumerator5")))
    (:`then_1`
      (if (`self.IsRunningRight`)
        (set `self.AniState` "NewEnumerator2")
        (`KismetSystemLibrary.Delay` 0.5)
        (set `self.AniState` "NewEnumerator0")))))

(event `Key|A`
  (params (Key :type "Key Structure"))
  ;[1 1 1] Animations
  (:`Pressed`
    (set `self.AniState` "NewEnumerator4")
    (set `self.IsRunningRight` false)
    (set `self.IsRunningLeft` true))
  (:`Released`
    (set `self.AniState` "NewEnumerator5")))

(event `Hoeing Animation`
  ;[1 1 1] Animations
  ;;[1 1 1] Hoe
  (`|ExecutionSequence`
    (:`then_0`
      (if (`self.IsRunningLeft`)
        (set `self.AniState` "NewEnumerator7")
        (`KismetSystemLibrary.Delay` 0.5)
        (set `self.AniState` "NewEnumerator5")))
    (:`then_1`
      (if (`self.IsRunningRight`)
        (set `self.AniState` "NewEnumerator3")
        (`KismetSystemLibrary.Delay` 0.5)
        (set `self.AniState` "NewEnumerator0")))))

(fn `GameEnd`
  (`GameplayStatics.OpenLevelBySoftObjectPtr` "/Game/Levels/EndScreen.EndScreen"))

(fn `Spawn Crops`)

(fn `UserConstructionScript`
  (bind (_returnvalue_x _returnvalue_y) (`KismetMathLibrary.BreakVector` (`self.K2_GetActorLocation`)))
  (`self.K2_SetActorLocation` (`KismetMathLibrary.MakeVector` _returnvalue_x _returnvalue_y 250.0)))